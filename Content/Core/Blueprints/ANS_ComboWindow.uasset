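; Anim notify state that marks the combo input window within attack animations.
; On begin it finds the AttackSystemComponent on the mesh owner and calls OpenComboWindow; on end it calls CloseComboWindow.
; The notify holds no state itself, leaving combo logic to that component.
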(fn ReceivedNotifyBegin
  (params (MeshComp :type Skeletal%20Mesh%20Component%20Object%20Reference) (Animation :type Anim%20Sequence%20Base%20Object%20Reference) (TotalDuration :type Float%20%28single-precision%29) (EventReference :type Anim%20Notify%20Event%20Reference%20Structure%20%28by%20ref%29))
  (bind _asattack_system_component (Utilities|Casting|CastToAttackSystemComponent (Actor|GetComponentbyClass (Components|GetOwner MeshComp) "/Script/RPG_Game.AttackSystemComponent")))
  (Class|AttackSystemComponent|OpenComboWindow _asattack_system_component)
  (return true))

(fn ReceivedNotifyEnd
  (params (MeshComp :type Skeletal%20Mesh%20Component%20Object%20Reference) (Animation :type Anim%20Sequence%20Base%20Object%20Reference) (EventReference :type Anim%20Notify%20Event%20Reference%20Structure%20%28by%20ref%29))
  (bind _asattack_system_component (Utilities|Casting|CastToAttackSystemComponent (Actor|GetComponentbyClass (Components|GetOwner MeshComp) "/Script/RPG_Game.AttackSystemComponent")))
  (Class|AttackSystemComponent|CloseComboWindow _asattack_system_component)
  (return true))