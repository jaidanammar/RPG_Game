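; BP_CombatDummy is a damageable target dummy that reacts to hits and dies.
; Any damage reduces clamped health, and a dead flag stops further processing once health reaches zero.
; Surviving hits play a random montage from HitAnims when hit reactions are enabled.
; Death enables skeletal mesh physics after a brief delay for a ragdoll, then destroys the actor, with debug prints on hit and ragdoll.
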(event Custom|PlayHitReact
  (bind _hitanims (Variables|Default|GetHitAnims))
  (bind _returnvalue (Utilities|Array|Length _hitanims))
  ;[0.15 0.15 0.15 0.5] PlayHitReact
  (if (Variables|Default|GetEnableHitReact)
    (if (> _returnvalue 0)
      (Animation|Montage|PlayMontage (Variables|Default|GetSkeletalMesh) (Utilities|Array|Get(acopy) _hitanims (Math|Random|RandomIntegerinRange 0 (- _returnvalue 1)))))))

(event Custom|Ragdoll
  ;[0.15 0.15 0.15 0.5] Ragdoll
  (Utilities|FlowControl|Delay 0.1)
  (Physics|SetSimulatePhysics (Variables|Default|GetSkeletalMesh) true)
  (Development|PrintText "Ragdoll Fired!")
  (Utilities|FlowControl|Delay 2.5)
  (Actor|DestroyActor))

(event EventBeginPlay
  ;[0.15 0.15 0.15 0.5] BeginPlay()
  (Variables|Default|SetIsDead false))

(event Game|Damage|EventAnyDamage
  (params (Damage :type Float%20%28single-precision%29) (DamageType :type Damage%20Type%20Object%20Reference) (InstigatedBy :type Controller%20Object%20Reference) (DamageCauser :type Actor%20Object%20Reference))
  ;[0.15 0.15 0.15 0.5] Any Damage
  (Development|PrintString "HIT")
  (if (not (Variables|Default|GetIsDead))
    (Variables|Default|SetCurrentHealth (Math|Float|Clamp(Float) (- (Variables|Default|GetCurrentHealth) Damage) 0.0 (Variables|Default|GetMaxHealth)))
    (if (<= (Variables|Default|GetCurrentHealth) 0.0)
      (Variables|Default|SetIsDead true)
      (CallFunction|Ragdoll)
      (else
        (CallFunction|PlayHitReact)))))

(fn ConstructionScript)